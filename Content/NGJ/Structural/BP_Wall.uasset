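; BP_Wall is a grid-snapped wall actor that can be placed and destroyed.
; PlaceWall spawns a copy on a 50-unit XY grid; Tick holds unfinished placement preview, snapping to a constant origin and setting empty materials on overlap checks.
; DamageWall reduces HP, throwing physics cube debris while health remains.
; At zero HP it destroys the static mesh, hides the Destructible component and applies damage to it.
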(event Custom|Place%20Wall
  (params (Transform :type Transform))
  (Game|SpawnActorfromClass "BP_Wall_C" (Math|Transform|MakeTransform (Math|Vector|MakeVector (Math|Float|SnapToGrid(Float) (.x (.location Transform)) 5e+01) (Math|Float|SnapToGrid(Float) (.y (.location Transform)) 5e+01) (.z (.location Transform))) (.rotation Transform) (.scale Transform)) "Undefined" 0 0))

(event Custom|Damage%20Wall
  (params (Damage :type Float%20%28single-precision%29) (NewParam :type BP%20Hammer%20Object%20Reference))
  (bind _destructible (Variables|Default|GetDestructible))
  (bind _output_get (Variables|Default|SetHPCur (- (Variables|Default|GetHPCur) Damage)))
  (if (<= _output_get 0.0)
    (Components|DestroyComponent (Variables|Default|GetStaticMesh))
    (Development|SetHiddeninGame _destructible true false)
    (Class|DestructibleComponent|ApplyDamage _destructible 1e+02 (Transformation|GetActorLocation NewParam) (Transformation|GetActorForwardVector NewParam) 2e+02)
    (else
      (for _index (range 0 4)
        (bind _returnvalue (AddComponent|AddStaticMeshComponent false (Math|Transform|MakeTransform (Transformation|GetActorLocation NewParam) "0, 0, 0" "0.200000,0.200000,0.200000")))
        (Components|StaticMesh|SetStaticMesh _returnvalue "/Game/NGJ/Art/Characters/Meshes/1x1_cube.1x1_cube")
        (Physics|SetSimulatePhysics _returnvalue true)
        (Physics|AddImpulse _returnvalue (Math|Vector|MakeVector (Math|Random|RandomFloatinRange 15.0 3e+01) (Math|Random|RandomFloatinRange 15.0 3e+01) (Math|Random|RandomFloatinRange 15.0 3e+01)) "None" true)))))

(event EventBeginPlay)

(event Collision|EventActorBeginOverlap
  (params (OtherActor :type Actor%20Object%20Reference)))

(event EventTick
  (params (DeltaSeconds :type Float%20%28single-precision%29))
  ;[1 1 1] Placement of walls mechanic, missing char input
  (Transformation|SetActorLocation (Math|Vector|MakeVector (Math|Float|SnapToGrid(Float) 0.0 5e+01) (Math|Float|SnapToGrid(Float) 0.0 5e+01) 0.0) false false)
  (if (Variables|Default|GetIsPlacing)
    (if (== (Utilities|Array|Length (Collision|GetOverlappingActors (Variables|Default|GetPlacementCollision) 0 :!class /Script/Engine.PrimitiveComponent)) 0)
      (Rendering|Material|SetMaterial (Variables|Default|GetStaticMesh) 0 0)
      (else
        (Rendering|Material|SetMaterial (Variables|Default|GetStaticMesh) 0 0)))))

(fn ConstructionScript)