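; BP_PrisonCell is a prison cell actor whose door slides open automatically two seconds after play begins.
; The OpenCell event plays a moving-door sound, then drives a timeline that lerps the Door's relative location sideways along Y.
; When the timeline finishes, a lock sound plays at the actor's location.
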(event Custom|OpenCell
  (Audio|PlaySoundatLocation "/Game/NGJ/Sounds/S_Moving_Door.S_Moving_Door" (Transformation|GetActorLocation))
  (bind _newtrack_0 (Timeline|Timeline_0 PlayFromStart)
    (:Update
      (Transformation|SetRelativeLocation (Variables|Default|GetDoor) (Math|Vector|Lerp(Vector) "160.000000,-70.000000, 0" "160.000000,60.000000, 0" _newtrack_0) false false))
    (:Finished
      (Audio|PlaySoundatLocation "/Game/NGJ/Sounds/S_Lock.S_Lock" (Transformation|GetActorLocation)))))

(event EventBeginPlay
  (Utilities|FlowControl|Delay 2.0)
  (CallFunction|OpenCell))

(event Collision|EventActorBeginOverlap
  (params (OtherActor :type Actor%20Object%20Reference)))

(event EventTick
  (params (DeltaSeconds :type Float%20%28single-precision%29)))

(fn ConstructionScript)