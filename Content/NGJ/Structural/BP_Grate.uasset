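; BP_Grate is a grate fixed by screws that comes loose and falls once they are all removed.
; On BeginPlay it registers itself as Master on the BP_Screw in each of its four child actor components.
; Each ScrewRemoved event decrements the screw count, and at zero the static mesh starts simulating physics.
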(event Custom|ScrewRemoved
  (bind _screws (Variables|Default|GetScrews))
  (Math|Integer|DecrementInt _screws
    (:%20%20
      (if (<= _screws 0)
        (Physics|SetSimulatePhysics (Variables|Default|GetStaticMesh) true)))))

(event EventBeginPlay
  (for _array_element (Utilities|Array|MakeArray (Variables|Default|GetChildActor) (Variables|Default|GetChildActor1) (Variables|Default|GetChildActor2) (Variables|Default|GetChildActor3))
    (bind _asbp_screw (Utilities|Casting|CastToBP_Screw (Variables|/Script/Engine.ChildActorComponent|GetChildActor _array_element)))
    (Variables|/Game/NGJ/Structural/BP_Screw.BP_Screw_C|SetMaster _asbp_screw self)))

(fn ConstructionScript)