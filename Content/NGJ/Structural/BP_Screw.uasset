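; BP_Screw is a screw that a player unscrews by twisting a hand holding a BP_Screwdriver.
; On overlap it swaps the held tool's mesh for its own Screwdriver mesh and tracks the hand.
; Tick adds only positive hand-roll increases to that mesh's yaw, with a delayed turning sound.
; At the rotation goal it notifies Master, releases the tool, and enables physics, with a drop sound on hits.
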(event Custom|Close
  (bind _asbp_screwdriver (Utilities|Casting|CastToBP_Screwdriver (stale Collision|EventActorEndOverlap OtherActor)))
  (Development|SetHiddeninGame (Variables|/Game/NGJ/Engine/Masters/BP_Interactible_Master.BP_Interactible_Master_C|GetStaticMesh _asbp_screwdriver) false false)
  (Variables|Default|SetHand 0)
  (Development|SetHiddeninGame (Variables|Default|GetScrewdriver) true false))

(event EventBeginPlay)

(event Collision|EventActorBeginOverlap
  (params (OtherActor :type Actor%20Object%20Reference))
  (if (Variables|Default|GetAttached)
    (bind _asbp_screwdriver (Utilities|Casting|CastToBP_Screwdriver OtherActor))
    (Utilities|IsValid (Variables|/Game/NGJ/Engine/Masters/BP_Interactible_Master.BP_Interactible_Master_C|GetAttachedTo _asbp_screwdriver)
      (:Is%20Valid
        (Development|SetHiddeninGame (Variables|Default|GetScrewdriver) false false)
        (bind _output_get (Variables|Default|SetHand (Variables|/Game/NGJ/Engine/Masters/BP_Interactible_Master.BP_Interactible_Master_C|GetAttachedTo _asbp_screwdriver)))
        (Development|SetHiddeninGame (Variables|/Game/NGJ/Engine/Masters/BP_Interactible_Master.BP_Interactible_Master_C|GetStaticMesh _asbp_screwdriver) true false)
        (Variables|Default|SetLast%20Rotation (Transformation|GetWorldRotation (Variables|/Game/NGJ/Engine/Masters/BP_MotionController.BP_MotionController_C|GetHandMesh _output_get)))))))

(event EventTick
  (params (DeltaSeconds :type Float%20%28single-precision%29))
  (bind _hand (Variables|Default|GetHand))
  (bind _handmesh (Variables|/Game/NGJ/Engine/Masters/BP_MotionController.BP_MotionController_C|GetHandMesh _hand))
  (if (Variables|Default|GetAttached)
    (Utilities|IsValid _hand
      (:Is%20Valid
        (if (> (- (.roll (Transformation|GetWorldRotation _handmesh)) (.roll (Variables|Default|GetLast%20Rotation))) 0.0)
          (Utilities|FlowControl|Sequence
            (:then_0
              (bind _output_get (Variables|Default|SetRotation (+ (Variables|Default|GetRotation) (- (.roll (Transformation|GetWorldRotation _handmesh)) (.roll (Variables|Default|GetLast%20Rotation))))))
              (Variables|Default|SetLast%20Rotation (Transformation|GetWorldRotation _handmesh))
              (Transformation|SetRelativeRotation (Variables|Default|GetScrewdriver) (Math|Rotator|MakeRotator -1.8e+02 0.0 (Variables|Default|GetRotation)) false false)
              (if (not (> (Variables|Default|GetRotationGoal) _output_get))
                (Default|ScrewRemoved (Variables|Default|GetMaster))
                (Variables|Default|SetAttached false)
                (CallFunction|Close)
                (Physics|SetSimulatePhysics (Variables|Default|GetStaticMesh) true)
                (Utilities|FlowControl|Delay 3.0)))
            (:then_1
              (Utilities|FlowControl|Delay 1.5)
              (Audio|PlaySoundatLocation "/Game/NGJ/Sounds/screwTurn.screwTurn" (Transformation|GetWorldLocation (Variables|/Game/NGJ/Engine/Masters/BP_MotionController.BP_MotionController_C|GetAttachPoint _hand))))))))))

(event Collision|EventHit
  (params (MyComp :type Primitive%20Component%20Object%20Reference) (Other :type Actor%20Object%20Reference) (OtherComp :type Primitive%20Component%20Object%20Reference) (bSelfMoved :type Boolean) (HitLocation :type Vector :default "0, 0, 0") (HitNormal :type Vector :default "0, 0, 0") (NormalImpulse :type Vector :default "0, 0, 0") (Hit :type Hit%20Result%20Structure%20%28by%20ref%29))
  (bind _screwdrop (Variables|Default|GetscrewDrop))
  (if (not (Audio|Components|Audio|IsPlaying _screwdrop))
    (Audio|Components|Audio|Play _screwdrop 0.0)))

(event Collision|EventActorEndOverlap
  (params (OtherActor :type Actor%20Object%20Reference))
  (bind _asbp_screwdriver (Utilities|Casting|CastToBP_Screwdriver OtherActor))
  (Development|SetHiddeninGame (Variables|/Game/NGJ/Engine/Masters/BP_Interactible_Master.BP_Interactible_Master_C|GetStaticMesh _asbp_screwdriver) false false)
  (Variables|Default|SetHand 0)
  (Development|SetHiddeninGame (Variables|Default|GetScrewdriver) true false))

(fn ConstructionScript)