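; BP_Lazer is a laser beam obstacle that sweeps back and forth or around, sized to whatever it hits.
; Each tick it traces the Visibility channel along the cylinder's negative right vector and scales the whole actor's Y axis from the hit distance.
; From BeginPlay, a restarting timeline interpolates Scene1's relative rotation between two rotator variables.
; The actor overlap event is empty, so this graph applies no effect on contact.
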(event EventBeginPlay
  (bind _newtrack_0 (Timeline|Timeline_0 Play)
    (:Update
      (Transformation|SetRelativeRotation (Variables|Default|GetScene1) (Math|Rotator|Lerp(Rotator) (Variables|Default|GetNewVar_0) (Variables|Default|GetNewVar_1) _newtrack_0) false false))
    (:Finished
      (if true
        (Timeline|Timeline_0 PlayFromStart)))))

(event Collision|EventActorBeginOverlap
  (params (OtherActor :type Actor%20Object%20Reference)))

(event EventTick
  (params (DeltaSeconds :type Float%20%28single-precision%29))
  (bind _returnvalue (Transformation|GetActorLocation))
  (bind _outhit (Collision|LineTraceByChannel _returnvalue (+ _returnvalue (* (Math|Vector|GetRightVector (Transformation|GetWorldRotation (Variables|Default|GetCylinder))) -1e+04)) "TraceTypeQuery1" false 0 "None"))
  (Transformation|SetActorScale3D (Math|Vector|MakeVector 1.0 (* (.distance _outhit) 0.01) 1.0)))

(fn ConstructionScript)