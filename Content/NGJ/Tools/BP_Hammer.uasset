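; BP_Hammer is a hammer tool that damages BP_Wall actors when it overlaps them, scaled by how fast its head moves.
; Each tick it stores the distance the Head component moved since the previous frame as Vel, without dividing by delta time.
; On overlap with a wall, it calls DamageWall with Vel as the damage and passes itself along.
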(event EventBeginPlay)

(event Collision|EventActorBeginOverlap
  (params (OtherActor :type Actor%20Object%20Reference))
  (bind _asbp_wall (Utilities|Casting|CastToBP_Wall OtherActor))
  (Default|DamageWall _asbp_wall (Variables|Default|GetVel) self))

(event EventTick
  (params (DeltaSeconds :type Float%20%28single-precision%29))
  (bind _head (Variables|Default|GetHead))
  (bind _returnvalue (Transformation|GetWorldLocation _head))
  (Variables|Default|SetVel (Math|Vector|VectorLength (- _returnvalue (Variables|Default|GetLast%20Loc))))
  (Variables|Default|SetLast%20Loc _returnvalue))

(fn ConstructionScript
  (|CallParentFunction))